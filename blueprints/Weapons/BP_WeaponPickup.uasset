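; BP_WeaponPickup is a world pickup actor that gives the player a weapon.
; Each tick it yaws its Weapon component toward the player camera, offset by 90 degrees, so the displayed weapon billboards without pitching or rolling.
; On overlap with a BP_FPSPlayer, it calls EquipWeapon with its WeaponToAquire value and destroys itself.
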(event Collision|EventActorBeginOverlap
  (params (OtherActor :type Actor%20Object%20Reference))
  (bind _asbp_fpsplayer (Utilities|Casting|CastToBP_FPSPlayer OtherActor))
  (Default|EquipWeapon _asbp_fpsplayer (Variables|WeaponPickup|GetWeapon%20to%20aquire))
  (Actor|DestroyActor))

(event EventTick
  (params (DeltaSeconds :type Float%20%28single-precision%29))
  (bind _weapon (Variables|Default|GetWeapon))
  (Transformation|SetWorldRotation _weapon (Math|Rotator|MakeRotator 0.0 0.0 (- (.yaw (Math|Rotator|FindLookatRotation (Transformation|GetWorldLocation _weapon) (Camera|GetCameraLocation (Game|GetPlayerCameraManager 0)))) 9e+01)) false false))

(fn ConstructionScript)