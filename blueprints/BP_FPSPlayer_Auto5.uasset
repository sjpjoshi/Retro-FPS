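; First-person player character that handles movement, mouse look and an equipped weapon.
; BeginPlay adds the weapon HUD, then EquipWeapon swaps the Weapon child actor's class, initializes it through IPlayerWeapon and plays its draw sequence.
; Tick drives the weapon's bobbing from whether the character is moving.
; Movement follows control yaw; the look axis names are crossed, with Up/Down feeding yaw and Right/Left feeding pitch.
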(event Custom|Equip%20Weapon
  (params (Weapon :type BP%20Player%20Weapon%20Base%20Class%20Reference))
  (bind _childactor (Variables|/Script/Engine.ChildActorComponent|GetChildActor (Variables|Default|GetWeapon)))
  ;[1 1 1] equip weapon
  (bind _output_get (Variables|Player|SetCurrentWeapon Weapon))
  (ChildActorComponent|SetChildActorClass (Variables|Default|GetWeapon) _output_get)
  (if (Utilities|DoesObjectImplementInterface _childactor "/Game/fps/blueprints/IPlayerWeapon.IPlayerWeapon_C")
    (Class|IPlayerWeapon|Initalizeweapon(Message) _childactor)
    (bind _asbp_player_weapon_base (Utilities|Casting|CastToBP_PlayerWeaponBase _childactor))
    (Sequencer|Player|Play (Variables|/Script/ActorSequence.ActorSequenceComponent|GetSequencePlayer (Variables|/Game/fps/blueprints/BP_PlayerWeaponBase.BP_PlayerWeaponBase_C|GetWeapon%20draw _asbp_player_weapon_base)) :!class /Script/MovieScene.MovieSceneSequencePlayer)))

(event EventBeginPlay
  ;[1 1 1] crosshair
  (bind _returnvalue (UserInterface|CreateWidget "/Game/fps/blueprints/WEP_HUD.WEP_HUD_C"))
  (UserInterface|Viewport|AddtoViewport _returnvalue 0)
  (CallFunction|EquipWeapon "/Game/fps/blueprints/BP_PlayerWeaponBase.BP_PlayerWeaponBase_C"))

(event EventTick
  (params (DeltaSeconds :type Float%20%28single-precision%29))
  (bind _asbp_player_weapon_base (Utilities|Casting|CastToBP_PlayerWeaponBase (Variables|/Script/Engine.ChildActorComponent|GetChildActor (Variables|Default|GetWeapon))))
  (Default|WeaponBobbing _asbp_player_weapon_base (> (Math|Vector|VectorLength (Variables|/Script/Engine.MovementComponent|GetVelocity (Variables|Character|GetCharacterMovement))) 0.0) DeltaSeconds))

(event Input|AxisEvents|InputAxisMoveForward/Backward
  (params (AxisValue :type Float%20%28single-precision%29))
  ;[1 1 1] movement section
  (Pawn|Input|AddMovementInput (Math|Vector|GetForwardVector (Math|Rotator|MakeRotator 0.0 0.0 (.yaw (Pawn|GetControlRotation :!class /Script/Engine.Pawn)))) AxisValue false))

(event Input|AxisEvents|InputAxisMoveRight/Left
  (params (AxisValue :type Float%20%28single-precision%29))
  ;[1 1 1] movement section
  (Pawn|Input|AddMovementInput (Math|Vector|GetRightVector (Math|Rotator|MakeRotator 0.0 0.0 (.yaw (Pawn|GetControlRotation :!class /Script/Engine.Pawn)))) AxisValue false))

(event Input|AxisEvents|InputAxisLookUp/DownMouse
  (params (AxisValue :type Float%20%28single-precision%29))
  ;[1 1 1] mouse look
  (Pawn|Input|AddControllerYawInput AxisValue))

(event Input|AxisEvents|InputAxisTurnRight/LeftMouse
  (params (AxisValue :type Float%20%28single-precision%29))
  ;[1 1 1] mouse look
  (Pawn|Input|AddControllerPitchInput AxisValue))

(fn ConstructionScript)