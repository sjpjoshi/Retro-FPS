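; BP_WeaponPickup is a world pickup that gives the player the weapon selected in its WeaponToAquire variable.
; The construction script sets the Item flipbook to match that weapon, pistol or rocket launcher, and clears it for NONE.
; When a BP_FPSPlayer overlaps it, the pickup passes the weapon to that player's PickupWeapon and destroys itself.
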(event Collision|EventActorBeginOverlap
  (params (OtherActor :type Actor%20Object%20Reference))
  (bind _asbp_fpsplayer (Utilities|Casting|CastToBP_FPSPlayer OtherActor))
  (Default|PickupWeapon _asbp_fpsplayer (Variables|WeaponPickup|GetWeapon%20to%20aquire))
  (Actor|DestroyActor))

(fn ConstructionScript
  (bind _item (Variables|Default|GetItem))
  (switch Utilities|FlowControl|Switch|SwitchonEnum_WeaponList (Variables|WeaponPickup|GetWeapon%20to%20aquire)
    (:NewEnumerator0
      (Sprite|SetFlipbook _item))
    (:NewEnumerator1
      (Sprite|SetFlipbook _item "/Game/fps/Flipbooks/FB_Pickups/FB_PistolPickup.FB_PistolPickup"))
    (:NewEnumerator2
      (Sprite|SetFlipbook _item "/Game/fps/Flipbooks/FB_Pickups/FB_Launcher_Pickup.FB_Launcher_Pickup"))))