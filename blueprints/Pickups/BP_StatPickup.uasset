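; BP_StatPickup is a health or armor pickup displayed as a flipbook.
; Its construction script uses pickup type and size to set the flipbook, item scale and matching gameplay tag.
; Full-health and full-armor checks read a base attribute from a given Ability System Component, adding or removing a Full tag on the pickup's tag container at the maximum of 100.
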(fn ConstructionScript
  (|CallParentFunction)
  (CallFunction|SetStatFBPickup))

(fn SetStatFBPickup
  (bind _item (Variables|Default|GetItem))
  (bind _enum_pickup_size (Variables|Default|GetEnum%20pickup%20size))
  (bind _item_2 (Variables|Default|GetItem))
  (switch Utilities|FlowControl|Switch|SwitchonEnum_Pickup_type (Variables|Default|GetPickup%20type)
    (:NewEnumerator0
      (Sprite|SetFlipbook _item "/Game/fps/Flipbooks/FB_Pickups/FB_Armor_Pickup.FB_Armor_Pickup")
      (switch Utilities|FlowControl|Switch|SwitchonEnum_Pickup_size _enum_pickup_size
        (:NewEnumerator0
          (Transformation|SetRelativeScale3D _item_2 "1.000000,1.000000,1.000000")
          (Variables|Default|SetPickup%20Tag "(GameplayTags=((TagName=\"Pickup.Armor.small\")))"))
        (:NewEnumerator1
          (Transformation|SetRelativeScale3D _item_2 "2.000000,2.000000,2.000000")
          (Variables|Default|SetPickup%20Tag "(GameplayTags=((TagName=\"Pickup.Armor.large\")))"))))
    (:NewEnumerator1
      (Sprite|SetFlipbook _item "/Game/fps/Flipbooks/FB_Pickups/FB_Health_Pickup.FB_Health_Pickup")
      (switch Utilities|FlowControl|Switch|SwitchonEnum_Pickup_size _enum_pickup_size
        (:NewEnumerator0
          (Transformation|SetRelativeScale3D _item_2 "1.000000,1.000000,1.000000")
          (Variables|Default|SetPickup%20Tag "(GameplayTags=((TagName=\"Pickup.Health.small\")))"))
        (:NewEnumerator1
          (Transformation|SetRelativeScale3D _item_2 "2.000000,2.000000,2.000000")
          (Variables|Default|SetPickup%20Tag "(GameplayTags=((TagName=\"Pickup.Health.large\")))"))))))

(fn FullHealthCheck
  (params (Ability%20System :type Ability%20System%20Component%20Object%20Reference))
  (bind _pickup_tag (Variables|Default|GetPickup%20Tag))
  (if (== (.ReturnValue (Class|AbilitySystemBlueprintLibrary|GetFloatAttributeBasefromAbilitySystemComponent Ability%20System "(AttributeName=\"Health\",Attribute=/Script/retrofps.RetroFPSAttributeSet:Health,AttributeOwner=Class'\"/Script/retrofps.RetroFPSAttributeSet\"')")) 1e+02)
    (GameplayTags|AddGameplayTag _pickup_tag "(TagName=\"Player.Health.Full\")" :!class /Script/GameplayTags.BlueprintGameplayTagLibrary)
    (else
      (GameplayTags|RemoveGameplayTag _pickup_tag "(TagName=\"Player.Health.Full\")" :!class /Script/GameplayTags.BlueprintGameplayTagLibrary))))

(fn FullArmorCheck
  (params (Ability%20System :type Ability%20System%20Component%20Object%20Reference))
  (bind _pickup_tag (Variables|Default|GetPickup%20Tag))
  (if (== (.ReturnValue (Class|AbilitySystemBlueprintLibrary|GetFloatAttributeBasefromAbilitySystemComponent Ability%20System "(AttributeName=\"Armor\",Attribute=/Script/retrofps.RetroFPSAttributeSet:Armor,AttributeOwner=Class'\"/Script/retrofps.RetroFPSAttributeSet\"')")) 1e+02)
    (GameplayTags|AddGameplayTag _pickup_tag "(TagName=\"Player.Armor.Full\")" :!class /Script/GameplayTags.BlueprintGameplayTagLibrary)
    (else
      (GameplayTags|RemoveGameplayTag _pickup_tag "(TagName=\"Player.Armor.Full\")" :!class /Script/GameplayTags.BlueprintGameplayTagLibrary))))