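; Retro FPS enemy character that shows a billboarded Paper2D sprite and runs a behavior tree through its AI controller.
; Each tick yaws the sprite toward the camera, then buckets the player's angle to its forward into five facings for walk or idle flipbooks.
; LeftSideVisible is computed, but left/right flipbook choice branches on IsWalking.
; Damage pauses directional updates for a hit flipbook; death disables capsule collision and plays dying, then dead.
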(event EventTick
  (params (DeltaSeconds :type Float%20%28single-precision%29))
  (Utilities|SpriteFacePlayer
    (:Out
      (if (not (or (Variables|Default|GetIs%20Dead) (Variables|Default|GetPause%20Angle%20Calculations)))
        (Utilities|GetEnemyAngle
          (:Out
            (Utilities|CheckifWalking
              (:Out
                (Utilities|CalculateFlipBook)))))))))

(event EventKillCharacter
  (bind _enemy (Variables|Components|GetEnemy))
  (|CallParentFunction)
  (Variables|Default|SetIs%20Dead true)
  (Collision|SetCollisionEnabled (Variables|Default|GetCapsuleComponent) "NoCollision")
  (Sprite|SetFlipbook _enemy (Variables|Default|GetDying))
  (Utilities|FlowControl|Delay (Class|PaperFlipbookComponent|GetFlipbookLength _enemy))
  (Sprite|SetFlipbook (Variables|Components|GetEnemy) (Variables|Default|GetDead)))

(event EventTakeDamage
  (params (Cue%20Data :type Gameplay%20Cue%20Parameters%20Structure))
  (bind _enemy (Variables|Components|GetEnemy))
  (|CallParentFunction Cue%20Data)
  (if (not (Variables|Default|GetIs%20Dead))
    (Variables|Default|SetPause%20Angle%20Calculations true)
    (Sprite|SetFlipbook _enemy (Variables|Default|GetDamaged))
    (Utilities|FlowControl|Delay (Class|PaperFlipbookComponent|GetFlipbookLength _enemy))
    (Variables|Default|SetPause%20Angle%20Calculations false)))

(event EventBeginPlay
  (bind _asbp_retro_fps_enemy_ai (Utilities|Casting|CastToBP_RetroFps_EnemyAI (Pawn|GetController)))
  (AI|RunBehaviorTree _asbp_retro_fps_enemy_ai (Variables|Default|GetBehavior%20Tree)))

(fn ConstructionScript)

(fn SetFlipbook
  (params (Walking :type Paper%20Flipbook%20Object%20Reference) (Idle :type Paper%20Flipbook%20Object%20Reference))
  (bind _enemy (Variables|Components|GetEnemy))
  (if (Variables|Default|GetIs%20Walking)
    (Sprite|SetFlipbook _enemy Walking)
    (else
      (Sprite|SetFlipbook _enemy Idle))))