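; Enemy AI for the retro FPS that turns AI Perception updates on Player-tagged actors into blackboard state.
; Sensing the player cancels any lost-sight timer, then sets the "Can see target" flag and the "Target Actor" key.
; Losing the player clears the flag at once but keeps the target until a delayed LostSight timer empties it, giving the enemy a short memory.
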(event OnTargetPerceptionUpdated(AIPerception)
  (params (Actor :type Actor%20Object%20Reference) (Stimulus :type AI%20Stimulus%20Structure))
  (bind _output_get (Variables|Default|SetPervieved%20Actor Actor))
  (if (Actor|ActorHasTag _output_get "Player")
    (if (.bsuccessfullysensed Stimulus)
      (Utilities|Time|ClearandInvalidateTimerbyHandle (Variables|Default|GetLost%20Sight%20Timer))
      (CallFunction|UpdatedSightKey true)
      (CallFunction|UpdatedTargetKey (Variables|Default|GetPervieved%20Actor))
      (else
        (bind _returnvalue (Utilities|Time|SetTimerbyEvent (delegate Custom|Lost%20Sight) 8.0))
        (Variables|Default|SetLost%20Sight%20Timer _returnvalue)
        (CallFunction|UpdatedSightKey false)))))

(event Custom|Lost%20Sight
  (CallFunction|UpdatedTargetKey))

(fn ConstructionScript)

(fn UpdatedSightKey
  (params (Has%20line%20of%20sight :type Boolean))
  (AI|Components|Blackboard|SetValueasBool (AI|GetBlackboard 0) (Utilities|Name|MakeLiteralName "Can see target") Has%20line%20of%20sight))

(fn UpdatedTargetKey
  (params (Target%20Actor :type Actor%20Object%20Reference))
  (AI|Components|Blackboard|SetValueasObject (AI|GetBlackboard 0) (Utilities|Name|MakeLiteralName "Target Actor") Target%20Actor))