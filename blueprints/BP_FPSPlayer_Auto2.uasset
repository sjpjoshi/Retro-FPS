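; First-person player pawn or character, judging by its name, that handles basic movement and mouse look and shows the WEP_HUD crosshair.
; BeginPlay creates the HUD widget and adds it to the viewport.
; Movement axes add input along forward and right vectors from control yaw only, so pitch does not affect direction.
; The look axis names appear swapped: Look Up / Down drives yaw and Turn Right / Left drives pitch.
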(event EventBeginPlay
  ;[1 1 1] crosshair
  (bind _returnvalue (UserInterface|CreateWidget "/Game/fps/blueprints/WEP_HUD.WEP_HUD_C"))
  (UserInterface|Viewport|AddtoViewport _returnvalue 0))

(event Input|AxisEvents|InputAxisMoveForward/Backward
  (params (AxisValue :type Float%20%28single-precision%29))
  ;[1 1 1] movement section
  (Pawn|Input|AddMovementInput (Math|Vector|GetForwardVector (Math|Rotator|MakeRotator 0.0 0.0 (.yaw (Pawn|GetControlRotation :!class /Script/Engine.Pawn)))) AxisValue false))

(event Input|AxisEvents|InputAxisMoveRight/Left
  (params (AxisValue :type Float%20%28single-precision%29))
  ;[1 1 1] movement section
  (Pawn|Input|AddMovementInput (Math|Vector|GetRightVector (Math|Rotator|MakeRotator 0.0 0.0 (.yaw (Pawn|GetControlRotation :!class /Script/Engine.Pawn)))) AxisValue false))

(event Input|AxisEvents|InputAxisLookUp/DownMouse
  (params (AxisValue :type Float%20%28single-precision%29))
  ;[1 1 1] mouse look
  (Pawn|Input|AddControllerYawInput AxisValue))

(event Input|AxisEvents|InputAxisTurnRight/LeftMouse
  (params (AxisValue :type Float%20%28single-precision%29))
  ;[1 1 1] mouse look
  (Pawn|Input|AddControllerPitchInput AxisValue))

(fn ConstructionScript)