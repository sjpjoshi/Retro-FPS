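; Base Gameplay Ability for firing a weapon in a retro FPS, with FireWeapon left for child classes to override.
; On activation it commits, listens for the weapon event tag, fires, then ends after the remaining cooldown.
; Received weapon events apply the weapon Gameplay Effect to the payload's target data.
; Ending cleans up the event and delay tasks, calling an empty Reset if the delay task is valid.
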(event Custom|waitForEvent
  ;[1 1 1] Wait for Gameplay Tag
  (bind (_asynctaskproxy _payload) (Ability|Tasks|WaitGameplayEvent (Variables|Default|GetWeapon%20Event%20Tag) 0)
    (:then
      (Variables|Default|SetGameplay%20Event%20wait%20Task _asynctaskproxy))
    (:EventReceived
      (GameplayEffects|ApplyGameplayEffectToTarget (.TargetData (Utilities|Struct|BreakGameplayEventData _payload)) (Variables|Default|GetWeapon%20%20Effect%20) 1 1))))

(event Custom|Fire%20Weapon)

(event Ability|EventActivateAbility
  ;[1 1 1] Activation
  (Ability|CommitAbility)
  (CallFunction|WaitforEvent)
  (CallFunction|FireWeapon)
  (bind _asynctaskproxy (Ability|Tasks|WaitDelay (Class|GameplayAbility|GetCooldownTimeRemaining))
    (:then
      (Variables|Default|SetFire%20Rate%20Delay%20Task _asynctaskproxy))
    (:OnFinish
      (Ability|EndAbility))))

(event Ability|EventOnEndAbility
  (params (bWasCancelled :type Boolean))
  (bind _gameplay_event_wait_task (Variables|Default|GetGameplay%20Event%20wait%20Task))
  (bind _fire_rate_delay_task (Variables|Default|GetFire%20Rate%20Delay%20Task))
  ;[1 1 1] end ability cleanup
  (Utilities|IsValid _gameplay_event_wait_task
    (:Is%20Valid
      (GameplayTasks|EndTask _gameplay_event_wait_task))
    (:Is%20Not%20Valid
      _))
  (Utilities|IsValid _fire_rate_delay_task
    (:Is%20Valid
      (GameplayTasks|EndTask _fire_rate_delay_task)
      (CallFunction|Reset))))

(fn Reset)